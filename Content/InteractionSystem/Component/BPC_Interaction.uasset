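; Character component that lets its owner use nearby BPI_Interactable actors through Press, Hold or multi-Tap input on IA_Interact.
; Capsule overlaps maintain an in-range list whose last entry is active and gets a screen-space WB_Interaction prompt.
; Hold binds dispatchers fed by the input action's ongoing and end events, while Tap counts presses, both updating widget progress.
; Triggering yaws the character toward the target and plays a montage whose "Interact" notify calls the interface.
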(event `self.ReceiveBeginPlay`
  ;[0.08305 1 0] Begin Play
  (`self.GetOwnerData`)
  (bind _returnvalue (`|AddComponentByClass` :`self` (`self.GetOwner`) :`Class` "/Script/UMG.WidgetComponent" :`bManualAttachment` true))
  (`WidgetComponent.SetWidgetSpace` _returnvalue "Screen")
  (`WidgetComponent.SetDrawSize` _returnvalue (250.0 30.0))
  (set `self.InteractionWidgetComponent` _returnvalue))

(event `GetOwnerData`
  ;[0 0 0] Access Owner's capsule component
  (bind _ascharacter (cast `Character` (`self.GetOwner`)))
  (set `self.As Character` _ascharacter)
  (bind _capsulecomponent (`Character.CapsuleComponent` _ascharacter))
  (add `PrimitiveComponent.OnComponentBeginOverlap` _capsulecomponent (`|CreateDelegate` :!event `HandleOverlapBegin`))
  (add `PrimitiveComponent.OnComponentEndOverlap` _capsulecomponent (`|CreateDelegate` :!event `HandleOverlapEnd`)))

(event `HandleOverlapBegin`
  (params (OverlappedComponent :type "PrimitiveComponent Object Reference") (OtherActor :type "Actor Object Reference") (OtherComp :type "PrimitiveComponent Object Reference") (OtherBodyIndex :type Integer) (bFromSweep :type Boolean) (SweepResult :type "HitResult Structure (by ref)"))
  ;[0 0 0] Handle overlap events
  (if (`KismetSystemLibrary.DoesImplementInterface` OtherActor "/Game/InteractionSystem/Interface/BPI_Interactable.BPI_Interactable_C")
    (`KismetArrayLibrary.Array_AddUnique` (`self.InteractablesInRange`) OtherActor)
    (`self.RenderInteractionWidget`)))

(event `HandleOverlapEnd`
  (params (OverlappedComponent :type "PrimitiveComponent Object Reference") (OtherActor :type "Actor Object Reference") (OtherComp :type "PrimitiveComponent Object Reference") (OtherBodyIndex :type Integer))
  ;[0 0 0] Handle overlap events
  (if (`KismetSystemLibrary.DoesImplementInterface` OtherActor "/Game/InteractionSystem/Interface/BPI_Interactable.BPI_Interactable_C")
    (if (== OtherActor (`self.GetActiveInteractable`))
      (`self.ResetInteractionState`))
    (`KismetArrayLibrary.Array_RemoveItem` (`self.InteractablesInRange`) OtherActor)
    (`self.RenderInteractionWidget`)))

(event `EnhancedInput|/Game/InteractionSystem/Input/IA_Interact`
  (params (ActionValue :type Boolean) (ElapsedSeconds :type "Float (double-precision)") (TriggeredSeconds :type "Float (double-precision)") (InputAction :type "InputAction Object Reference" :default "/Game/InteractionSystem/Input/IA_Interact.IA_Interact"))
  ;[0 0 0] Make sure to have IA_Interact on owner's IMC
  (:`Started`
    (`self.InteractBegin`))
  (:`Ongoing`
    (`self.OnInteractionPressOngoing` ElapsedSeconds))
  (:`Canceled`
    (clear `self.OnInteractionPressOngoing` :!label _label)
    (`self.OnInteractionEnded`))
  (:`Completed`
    (goto _label)))

(event `InteractBegin`
  (bind _active_interactable (`self.GetActiveInteractable`))
  ;[0 0 0] Make sure to have IA_Interact on owner's IMC
  (`/Engine/EditorBlueprintResources/StandardMacros.IsValid` _active_interactable
    (:`Is Valid`
      (bind _type (message `/Game/InteractionSystem/Interface/BPI_Interactable.Get_Interaction Type` _active_interactable))
      (switch `/Game/InteractionSystem/Variables/E_InteractionType` _type
        (:`NewEnumerator0`
          (`self.InteractWithActiveInteractable`))
        (:`NewEnumerator1`
          (add `self.OnInteractionPressOngoing` (`|CreateDelegate` :!event `HandleInteractionHoldOngoing`))
          (add `self.OnInteractionEnded` (`|CreateDelegate` :!event `HandleInteractionEnded`)))
        (:`NewEnumerator2`
          (`self.InteractionTap`))))))

(event `InteractionTap`
  ;[0 0 0] Make sure to have IA_Interact on owner's IMC
  (`GameplayStatics.PlaySound2D` "/Engine/VREditor/Sounds/UI/Gizmo_Handle_Clicked.Gizmo_Handle_Clicked" 1.0 1.0 0.0 null null)
  (`/Engine/EditorBlueprintResources/StandardMacros.IncrementInt` (`self.CurrentTapCount`)
    (:`  `
      (bind _value (message `/Game/InteractionSystem/Interface/BPI_Interactable.Get_TapCount` (`self.GetActiveInteractable`)))
      (if (<= _value 0)
        (`self.InteractWithActiveInteractable`)
        (else
          (bind _interactionwidgetref (`self.InteractionWidgetRef`)
            (:`then`
              (`/Game/InteractionSystem/Widgets/WB_Interaction.SetProgressPercent` _interactionwidgetref (/ (`self.CurrentTapCount`) _value))
              (if (>= (`self.CurrentTapCount`) _value)
                (`self.InteractWithActiveInteractable`)))
            (:`else`)))))))

(event `HandleInteractionEnded`
  ;[0 0 0] Make sure to have IA_Interact on owner's IMC
  (bind _interactionwidgetref (`self.InteractionWidgetRef`)
    (:`then`
      (`/Game/InteractionSystem/Widgets/WB_Interaction.SetProgressPercent` _interactionwidgetref 0.0)
      (remove `self.OnInteractionEnded` (delegate `HandleInteractionEnded`)))
    (:`else`)))

(event `HandleInteractionHoldOngoing` :!signature `self.OnInteractionPressOngoing`
  (params (ElapsedSeconds :type "Float (double-precision)"))
  (bind _active_interactable (`self.GetActiveInteractable`))
  ;[0 0 0] Make sure to have IA_Interact on owner's IMC
  (`/Engine/EditorBlueprintResources/StandardMacros.IsValid` _active_interactable
    (:`Is Valid`
      (bind _duration (message `/Game/InteractionSystem/Interface/BPI_Interactable.Get_HoldDuration` _active_interactable))
      (bind _interactionwidgetref (`self.InteractionWidgetRef`)
        (:`then`
          (`/Game/InteractionSystem/Widgets/WB_Interaction.SetProgressPercent` _interactionwidgetref (/ ElapsedSeconds _duration)))
        (:`else`
          _))
      (if (> ElapsedSeconds _duration)
        (`self.InteractWithActiveInteractable`)
        (remove `self.OnInteractionPressOngoing` (delegate `HandleInteractionHoldOngoing`))))))

(event `InteractWithActiveInteractable`
  (bind _as_character (`self.As Character`))
  (bind (_returnvalue_roll _returnvalue_pitch _returnvalue_yaw) (`KismetMathLibrary.BreakRotator` (`KismetMathLibrary.FindLookAtRotation` (`Actor.K2_GetActorLocation` _as_character) (`self.GetActiveInteractableLocation`))))
  ;[0 0 0] Interact With Active Interactable
  (`/Engine/EditorBlueprintResources/StandardMacros.IsValid` (`self.GetActiveInteractable`)
    (:`Is Valid`
      (`Actor.K2_SetActorRotation` _as_character (`KismetMathLibrary.MakeRotator` 0.0 0.0 _returnvalue_yaw) false)
      (bind _notifyname (`|PlayMontage` (`Character.Mesh` (`self.As Character`)) "/Game/InteractionSystem/Animations/Montages/Opening_UE_Montage.Opening_UE_Montage")
        (:`OnNotifyBegin`
          (if (== _notifyname "Interact")
            (message `/Game/InteractionSystem/Interface/BPI_Interactable.Interact` (`self.GetActiveInteractable`) (`self.GetOwner`))
            (`self.ResetInteractionState`)
            (`self.RenderInteractionWidget`)))))))

(fn `GetActiveInteractable`
  (returns (`Active Interactable` :type "Actor Object Reference"))
  (bind _interactablesinrange (`self.InteractablesInRange`))
  (return (`|GetArrayItem` _interactablesinrange (`KismetArrayLibrary.Array_LastIndex` _interactablesinrange))))

(fn `GetActiveInteractableLocation`
  (returns (Location :type "Vector Structure"))
  (bind _active_interactable (`self.GetActiveInteractable`))
  (`/Engine/EditorBlueprintResources/StandardMacros.IsValid` _active_interactable
    (:`Is Valid`
      (bind _location (message `/Game/InteractionSystem/Interface/BPI_Interactable.Get_InteractionLocation` _active_interactable))
      (return (`KismetMathLibrary.SelectVector` (`Actor.K2_GetActorLocation` _active_interactable) _location (`KismetMathLibrary.Vector_IsZero` _location))))))

(fn `RenderInteractionWidget`
  (bind _active_interactable (`self.GetActiveInteractable`))
  (`/Engine/EditorBlueprintResources/StandardMacros.IsValid` _active_interactable
    (:`Is Valid`
      (bind _type (message `/Game/InteractionSystem/Interface/BPI_Interactable.Get_Interaction Type` _active_interactable))
      (bind _prompt (message `/Game/InteractionSystem/Interface/BPI_Interactable.Get_InteractionPrompt` _active_interactable))
      (bind _returnvalue (`|CreateWidget` "/Game/InteractionSystem/Widgets/WB_Interaction.WB_Interaction_C" null _type _prompt))
      (set `self.InteractionWidgetRef` _returnvalue)
      (`WidgetComponent.SetWidget` (`self.InteractionWidgetComponent`) _returnvalue)
      (`SceneComponent.K2_SetWorldLocation` (`self.InteractionWidgetComponent`) (`self.GetActiveInteractableLocation`) false false))
    (:`Is Not Valid`
      (`WidgetComponent.SetWidget` (`self.InteractionWidgetComponent`) null))))

(fn `ResetInteractionState`
  (remove `self.OnInteractionPressOngoing` (`|CreateDelegate` :!event `HandleInteractionHoldOngoing`))
  (set `self.CurrentTapCount` 0))