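; BP_Door is an interactable door that swings open or shut with a sound on each interaction.
; Interact checks IsOpen and calls OpenDoor or CloseDoor, which play or reverse one timeline driving the door's yaw.
; Getters supply the interaction system with type, location, hold duration, tap count and prompt.
; The prompt selection looks inverted, reading "to open the door" while IsOpen is true.
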(event `self.ReceiveBeginPlay`)

(event `/Game/InteractionSystem/Interface/BPI_Interactable.Interact`
  (params (Interactor :type "Actor Object Reference"))
  ;[0 0 0] Event Interact
  (if (`self.IsOpen`)
    (`self.CloseDoor`)
    (else
      (`self.OpenDoor`))))

(event `OpenDoor`
  ;[0 0 0] Open & Close
  (set `self.IsOpen` true)
  (`GameplayStatics.PlaySoundAtLocation` (`self.OpeningSound`) (`self.K2_GetActorLocation`) (struct) 1.0 1.0 0.0 null null null null)
  (bind (_direction _zrotation) (`Timeline|OpenDoorTimeline` :!label _label)
    (:`Update`
      (`SceneComponent.K2_SetRelativeRotation` (`self.Door`) (`KismetMathLibrary.MakeRotator` 0.0 0.0 _zrotation) false false))))

(event `CloseDoor`
  ;[0 0 0] Open & Close
  (set `self.IsOpen` false)
  (`GameplayStatics.PlaySoundAtLocation` (`self.ClosingSound`) (`self.K2_GetActorLocation`) (struct) 1.0 1.0 0.0 null null null null)
  (goto _label :!via `Reverse`))

(fn `Get_HoldDuration`
  (returns (Duration :type "Float (double-precision)"))
  (return 0.0))

(fn `Get_Interaction Type`
  (returns (Type :type "/Game/InteractionSystem/Variables/E_InteractionType Enum"))
  (return (`self.Interaction Type`)))

(fn `Get_InteractionLocation`
  (returns (Location :type "Vector Structure"))
  (return (`SceneComponent.K2_GetComponentLocation` (`self.Interaction Location`))))

(fn `Get_InteractionPrompt`
  (returns (Prompt :type Text))
  (return (`KismetMathLibrary.SelectText` "to open the door" "to close the door" (`self.IsOpen`))))

(fn `Get_TapCount`
  (returns (Value :type Integer))
  (return 4))

(fn `UserConstructionScript`)