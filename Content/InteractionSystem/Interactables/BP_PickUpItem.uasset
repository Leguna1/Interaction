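; Pickup item actor for the interaction system that removes itself from the world when interacted with.
; On Interact it prints a message naming the item and the interactor, plays a pickup sound at its location and destroys itself; no inventory is actually updated.
; Interaction getters expose its hold duration and interaction type variables, while location, prompt and tap count return empty defaults.
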(event `/Game/InteractionSystem/Interface/BPI_Interactable.Interact`
  (params (Interactor :type "Actor Object Reference"))
  (`KismetSystemLibrary.PrintString` (`KismetTextLibrary.Conv_TextToString` (`|FormatText` "Added {itemName} to inventory of {ActorName}" (`KismetSystemLibrary.GetDisplayName` self) Interactor)) true true (struct :`G` 0.66 :`B` 1.0 :`A` 1.0) 10.0)
  (`GameplayStatics.PlaySoundAtLocation` (`self.PickUpSound`) (`self.K2_GetActorLocation`) (struct) 1.0 1.0 0.0 null null null null)
  (`self.K2_DestroyActor`))

(fn `Get_HoldDuration`
  (returns (Duration :type "Float (double-precision)"))
  (return (`self.Hold Duration`)))

(fn `Get_Interaction Type`
  (returns (Type :type "/Game/InteractionSystem/Variables/E_InteractionType Enum"))
  (return (`self.Interaction Type`)))

(fn `Get_InteractionLocation`
  (returns (Location :type "Vector Structure"))
  (return (0.0 0.0 0.0)))

(fn `Get_InteractionPrompt`
  (returns (Prompt :type Text))
  (return ""))

(fn `Get_TapCount`
  (returns (Value :type Integer))
  (return 0))

(fn `UserConstructionScript`)