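; Interactable NPC for the interaction system, showing a "to talk" prompt and playing a reaction when interacted with.
; On Interact it turns on yaw to face the interactor, then plays a sound at its location and a chicken dance montage on its mesh.
; Getter functions supply the interaction type, hold duration, prompt and world-space interaction location, with tap count fixed at zero.
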(event `/Game/InteractionSystem/Interface/BPI_Interactable.Interact`
  (params (Interactor :type "Actor Object Reference"))
  (bind (_returnvalue_roll _returnvalue_pitch _returnvalue_yaw) (`KismetMathLibrary.BreakRotator` (`KismetMathLibrary.FindLookAtRotation` (`self.K2_GetActorLocation`) (`self.K2_GetActorLocation` Interactor))))
  (`self.K2_SetActorRotation` (`KismetMathLibrary.MakeRotator` 0.0 0.0 _returnvalue_yaw))
  (`GameplayStatics.PlaySoundAtLocation` "/Engine/VREditor/Sounds/UI/Enter_Play.Enter_Play" (`self.K2_GetActorLocation`) (struct) 1.0 1.0 0.0 null null null null)
  (`|PlayMontage` (`self.Mesh`) "/Game/InteractionSystem/Animations/Montages/ChickenDance_UE_Montage.ChickenDance_UE_Montage"))

(fn `Get_HoldDuration`
  (returns (Duration :type "Float (double-precision)"))
  (return (`self.Hold Duration`)))

(fn `Get_InteractableType`
  (returns (InteractableType :type "/Game/InteractionSystem/Variables/E_InteractableType Enum"))
  (return (`self.Interactable Type`)))

(fn `Get_Interaction Type`
  (returns (Type :type "/Game/InteractionSystem/Variables/E_InteractionType Enum"))
  (return (`self.Type`)))

(fn `Get_InteractionLocation`
  (returns (Location :type "Vector Structure"))
  (return (`SceneComponent.K2_GetComponentLocation` (`self.InteractionLocation`))))

(fn `Get_InteractionPrompt`
  (returns (Prompt :type Text))
  (return "to talk"))

(fn `Get_TapCount`
  (returns (Value :type Integer))
  (return 0))

(fn `UserConstructionScript`)